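; Base weapon actor that supplies melee damage, hit collision and per-action montages for a combat character.
; On equip, it registers as main weapon with the owner's combat component and points its collision component at the item mesh, ignoring the owner.
; Collision hits apply point damage along the owner's forward vector.
; Montages are chosen by gameplay tag for light attack, dodge and death; helpers toggle collision, combat state and mesh physics.
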(event OnHit(BP_MainCollisionComponent)
  (params (HitResult :type Hit%20Result%20Structure))
  (CallFunction|OnHit HitResult))

(event Custom|SimulateWeaponPhysics
  (Collision|SetCollisionProfileName (CallFunction|GetItemMesh) "PhysicsActor" true :!class /Script/Engine.PrimitiveComponent)
  (Physics|SetSimulatePhysics (CallFunction|GetItemMesh) true))

(event Custom|ToggleCombat
  (params (bEnableCombat? :type Boolean))
  (Default|SetCombatEnable (Variables|Default|GetBP_CombatComponent) bEnableCombat?))

(fn ConstructionScript
  (|CallParentFunction))

(fn OnEquipped
  (|CallParentFunction)
  (Variables|Default|SetBP_CombatComponent (Actor|GetComponentbyClass (Components|GetOwner) "/Game/_Main/Blueprints/Components/BPC_CombatComponent.BPC_CombatComponent_C"))
  (Default|SetMainWeapon (Variables|Default|GetBP_CombatComponent) self)
  (Default|SetCollisionMeshComponent (Variables|Default|GetBP_MainCollisionComponent) (Variables|Default|GetItemStaticMesh))
  (Default|AddIgnoreActor (Variables|Default|GetBP_MainCollisionComponent) (Components|GetOwner)))

(fn OnHit
  (params (Hit :type Hit%20Result%20Structure%20%28by%20ref%29))
  (Game|Damage|ApplyPointDamage (.HitActor (Collision|BreakHitResult Hit)) (Stats|GetDamage) (Transformation|GetActorForwardVector (Components|GetOwner)) Hit (Game|GetInstigatorController) self "/Script/Engine.DamageType"))

(fn GetActionMontages
  (params (CharacterAction :type Gameplay%20Tag%20Structure))
  (|SwitchGameplayTag CharacterAction
    (:Character.Action.Attack.Light%20Attack
      (return (Variables|Animations|GetLightAttackMontages)))
    (:Character.Action.Dodge
      (return (Variables|Animations|GetDodgeMontages)))
    (:Character.Action.Die
      (return (Variables|Animations|GetDieMontages)))))

(fn GetDamage
  (return (Variables|Stats|GetDamage)))

(fn ActivateCollision
  (Default|ActivateCollision (Variables|Default|GetBP_MainCollisionComponent)))

(fn DeactivateCollision
  (Default|DeactivateCollision (Variables|Default|GetBP_MainCollisionComponent)))