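; Base equippable item actor that tracks its equipped state and attaches to its owning Character.
; On equip it sets the flag and snaps to AttachSocketName on the owner's mesh, while unequip only clears the flag without detaching.
; GetItemMesh returns the static mesh component if it has a valid mesh, otherwise the skeletal one.
; It also exposes its owned gameplay tags with an exact-match query.
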(event EventBeginPlay)

(event Collision|EventActorBeginOverlap
  (params (OtherActor :type Actor%20Object%20Reference)))

(event EventTick
  (params (DeltaSeconds :type Float%20%28single-precision%29)))

(fn ConstructionScript)

(fn AttachActor
  (params (SocketName :type Name))
  (Transformation|AttachComponentToComponent (Variables|/Script/Engine.Character|GetMesh (.AsCharacter (Utilities|Casting|CastToCharacter (Components|GetOwner)))) SocketName "SnapToTarget" "SnapToTarget" "SnapToTarget" true))

(fn GetItemMesh
  (Variables|/Script/Engine.StaticMeshComponent|GetStaticMesh (Variables|Default|GetItemStaticMesh)
    (:then
      (return (Variables|Default|GetItemStaticMesh)))
    (:else
      (return (Variables|Default|GetItemSkeletalMesh)))))

(fn OnEquipped
  (Variables|Default|SetbIsEquipped? true)
  (ItemMesh|AttachActor (Variables|Initialization|GetAttach%20Socket%20Name)))

(fn OnUnequipped
  (if (Variables|Default|GetbIsEquipped?)
    (Variables|Default|SetbIsEquipped? false)))

(fn SetIsEquipped
  (params (bIsEquipped? :type Boolean))
  (Variables|Default|SetbIsEquipped? bIsEquipped?))

(fn IsEquipped?
  (return (Variables|Default|GetbIsEquipped?)))

(fn GetOwnedGameplayTags
  (return (Variables|GameplayTags|GetOwnedGameplayTags)))

(fn HasMatchingGameplayTag
  (params (TagToCheck :type Gameplay%20Tag%20Structure))
  (return (GameplayTags|HasTag (Variables|GameplayTags|GetOwnedGameplayTags) TagToCheck true)))