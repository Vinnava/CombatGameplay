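; Base AI controller for enemy characters that runs each pawn's behavior tree on possession, unless it is a dummy.
; AI perception sets the blackboard Target from sensed player-tagged actors via sight or damage, clearing it when sight fails or finds a non-player.
; Combat toggles from the pawn's combat component and a can-attack event are mirrored into blackboard bools for the tree.
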(event OnPerceptionUpdated(AIPerception)
  (params (UpdatedActors :type Array%20of%20Actor%20Object%20References))
  (if (not (Variables|/Game/_Main/Blueprints/Character/Enemy/BPCH_EnemyBase.BPCH_EnemyBase_C|GetbIsDummy? (Variables|Default|GetMaster%20AI)))
    (CallFunction|UpdatePerception UpdatedActors)))

(event Custom|OnToggleCombat%20AI
  (params (bCombatEnable? :type Boolean))
  (CallFunction|SetBlackboardCombatEnable bCombatEnable?))

(event Custom|ToogleCanAttack
  (params (CanAttack :type Boolean))
  (if (not (Variables|/Game/_Main/Blueprints/Character/Enemy/BPCH_EnemyBase.BPCH_EnemyBase_C|GetbIsDummy? (Variables|Default|GetMaster%20AI)))
    (AI|Components|Blackboard|SetValueasBool (Variables|Default|GetBlackboard) (Utilities|Name|MakeLiteralName "bCanAttack") CanAttack)))

(event EventPossess
  (params (PossessedPawn :type Pawn%20Object%20Reference))
  (bind _asbpch_enemy_base (Utilities|Casting|CastToBPCH_EnemyBase PossessedPawn))
  (bind _output_get (Variables|Default|SetMaster%20AI _asbpch_enemy_base))
  (if (not (Variables|/Game/_Main/Blueprints/Character/Enemy/BPCH_EnemyBase.BPCH_EnemyBase_C|GetbIsDummy? _output_get))
    (EventDispatchers|BindEventtoOnToggleCombat (Variables|/Game/_Main/Blueprints/Character/Base/BPCH_Base.BPCH_Base_C|GetCombatComponent (Variables|Default|GetMaster%20AI)) (delegate Custom|OnToggleCombat%20AI))
    (AI|RunBehaviorTree (Variables|/Game/_Main/Blueprints/Character/Enemy/BPCH_EnemyBase.BPCH_EnemyBase_C|GetBehavior%20Tree (Variables|Default|GetMaster%20AI)))))

(fn ConstructionScript)

(fn UpdatePerception
  (params (PerceivedActors :type Array%20of%20Actor%20Object%20References))
  (for _array_element PerceivedActors
    (bind _output_get (LocalVariables|SetTheSensedActor _array_element))
    (bind _info (Class|AIPerceptionComponent|GetActorsPerception (Variables|Default|GetAIPerception) _output_get))
    (for (_array_element_2 _array_index) (.LastSensedStimuli (Utilities|Struct|BreakActorPerceptionBlueprintInfo _info))
      (LocalVariables|SetLastStimuli _array_element_2)
      (switch int _array_index ; 0: AI sight\n1: AI damage sense
        (:0
          (if (.bSuccessfullySensed (Utilities|Struct|BreakAIStimulus (LocalVariables|GetLastStimuli)))
            (bind _returnvalue (Class|GameplayTagBPI|HasMatchingGameplayTag(Message) _output_get "(TagName=\"Character.Player\")"))
            (if _returnvalue
              (CallFunction|SetBlackboardTargetActor (LocalVariables|GetTheSensedActor))
              (else
                (CallFunction|SetBlackboardTargetActor :!label _label)))
            (else
              (goto _label))))
        (:1
          (if (.bSuccessfullySensed (Utilities|Struct|BreakAIStimulus (LocalVariables|GetLastStimuli)))
            (bind _returnvalue_2 (Class|GameplayTagBPI|HasMatchingGameplayTag(Message) (LocalVariables|GetTheSensedActor) "(TagName=\"Character.Player\")"))
            (if _returnvalue_2
              (CallFunction|SetBlackboardTargetActor (LocalVariables|GetTheSensedActor)))))))))

(fn SetBlackboardTargetActor
  (params (NewTargetActor :type Actor%20Object%20Reference))
  (AI|Components|Blackboard|SetValueasObject (Variables|Default|GetBlackboard) (Utilities|Name|MakeLiteralName "Target") NewTargetActor))

(fn SetBlackboardCombatEnable
  (params (BoolValue :type Boolean))
  (AI|Components|Blackboard|SetValueasBool (Variables|Default|GetBlackboard) (Utilities|Name|MakeLiteralName "bCombatEnable") BoolValue))