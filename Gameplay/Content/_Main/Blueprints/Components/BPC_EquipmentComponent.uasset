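; BPC_EquipmentComponent is an actor component that spawns and tracks its owner's starting equipment.
; InitializeEquipment spawns each valid StartingEquipments class at the owner's transform with the owner as Owner and Instigator, calls OnEquipped, and adds it to CurrentEquipments.
; After each spawn it also enables combat on the main weapon from the owner's BPC_CombatComponent.
; GetCurrentEquipments exposes the spawned list.
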(fn InitializeEquipment
  (bind _returnvalue (Components|GetOwner))
  (for _array_element (Variables|Initialization|GetStartingEquipments)
    (if (Utilities|IsValidClass _array_element)
      (bind _returnvalue_2 (Game|SpawnActorfromClass _array_element (Transformation|GetActorTransform _returnvalue) "Undefined" "SelectDefaultAtRuntime" _returnvalue (.AsPawn (Utilities|Casting|CastToPawn _returnvalue))))
      (Default|OnEquipped _returnvalue_2)
      (Utilities|Array|AddUnique (Variables|Default|GetCurrentEquipments) _returnvalue_2)
      (Default|ToggleCombat (Default|GetMainWeapon (Actor|GetComponentbyClass _returnvalue "/Game/_Main/Blueprints/Components/BPC_CombatComponent.BPC_CombatComponent_C")) true)))
  (return))

(fn GetCurrentEquipments
  (return (Variables|Default|GetCurrentEquipments)))