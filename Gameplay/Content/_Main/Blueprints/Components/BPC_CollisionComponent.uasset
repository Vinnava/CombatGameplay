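; Actor component that detects hits along a mesh between two sockets while collision is activated.
; Each tick it runs a multi-sphere object trace between the socket locations, skipping ignored actors and those with exact-match ignored gameplay tags.
; New hit actors are recorded and broadcast through OnHit, so each is reported once per activation, as activating clears the list.
; Helper functions expose hit state and manage the ignore list.
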(event Custom|Activate%20Collision
  ;[0.05098 0.05098 0.05098] Enable Collision
  (CallFunction|ClearHitActors)
  (Variables|Default|SetbIsCollisionEnable? true))

(event Custom|Deactivate%20Collision
  ;[0.05098 0.05098 0.05098] Disable Collision
  (Variables|Default|SetbIsCollisionEnable? false))

(event Custom|Collision%20Trace
  (bind _collisionmeshcomponent (Variables|Default|GetCollisionMeshComponent))
  ;[0.05098 0.05098 0.05098] Collision Trace
  (bind _outhits (Collision|MultiSphereTraceForObjects (Transformation|GetSocketLocation _collisionmeshcomponent (Variables|Inittialization|GetStartSocketName)) (Transformation|GetSocketLocation _collisionmeshcomponent (Variables|Inittialization|GetEndSocketName)) (Variables|Inittialization|GetTraceRadius) (Variables|Inittialization|GetCollisionObjectType) false (Variables|Inittialization|GetActors%20to%20Ignore) (Variables|Inittialization|GetDraw%20Debug%20Type)))
  (for _array_element _outhits
    (bind _output_get (Variables|Default|SetLastHitResult _array_element))
    (bind _returnvalue (Class|GameplayTagBPI|GetOwnedGameplayTags(Message) (.HitActor (Collision|BreakHitResult _output_get))))
    (if (and (not (Utilities|Array|ContainsItem (Variables|Default|GetAlreadyHitActors) (.HitActor (Collision|BreakHitResult _output_get)))) (not (GameplayTags|HasAnyTags _returnvalue (Variables|Inittialization|GetIgnoreGameplayTags) true)))
      (bind _output_get_2 (Variables|Default|SetLastHitActor (.HitActor (Collision|BreakHitResult _output_get))))
      (Utilities|Array|Add (Variables|Default|GetAlreadyHitActors) _output_get_2)
      (Default|CallOnHit (Variables|Default|GetLastHitResult)))))

(event Custom|Clear%20Hit%20Actors
  ;[0.05098 0.05098 0.05098] Clear Hit Actors
  (Utilities|Array|Clear (Variables|Default|GetAlreadyHitActors)))

(event Custom|SetCollisionMeshComponent
  (params (CollisionMeshComponent :type Primitive%20Component%20Object%20Reference))
  ;[0.05098 0.05098 0.05098] Set Collision Mesh Component
  (Variables|Default|SetCollisionMeshComponent CollisionMeshComponent))

(event EventTick
  (params (DeltaSeconds :type Float%20%28single-precision%29))
  ;[0.05098 0.05098 0.05098] Tick
  (if (Variables|Default|GetbIsCollisionEnable?)
    (CallFunction|CollisionTrace)))

(fn IsCollisionEnabled?
  (return (Variables|Default|GetbIsCollisionEnable?)))

(fn GetAlreadyHitActors
  (return (Variables|Default|GetAlreadyHitActors)))

(fn GetLastHitResult
  (return (Variables|Default|GetLastHitResult)))

(fn GetCollisionMeshComponent
  (return (Variables|Default|GetCollisionMeshComponent)))

(fn GetIgnoreActors
  (return (Variables|Inittialization|GetActors%20to%20Ignore)))

(fn AddIgnoreActor
  (params (InActor :type Actor%20Object%20Reference%20%28by%20ref%29))
  (Utilities|Array|AddUnique (Variables|Inittialization|GetActors%20to%20Ignore) InActor))

(fn RemoveIgnoreActor
  (params (InActor :type Actor%20Object%20Reference%20%28by%20ref%29))
  (Utilities|Array|RemoveItem (Variables|Inittialization|GetActors%20to%20Ignore) InActor))