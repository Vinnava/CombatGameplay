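; Combat component that holds its owner's main weapon, combat-enabled flag and attack-chain state.
; Setting a new main weapon unequips and destroys the previous one before storing the replacement.
; Toggling combat broadcasts OnToggleCombat, noted as driving the AI controller's bCombatEnable blackboard key; a direct anim-instance update is left disconnected.
; ResetAttack clears the attack count, saved-attack and can-continue flags.
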(fn SetMainWeapon
  (params (NewWeapon :type BP%20Base%20Weapon%20Object%20Reference))
  (Utilities|FlowControl|Sequence
    (:then_0
      (bind _mainweapon (Variables|Default|GetMainWeapon)
        (:then
          (Default|OnUnequipped _mainweapon)
          (Actor|DestroyActor _mainweapon))
        (:else)))
    (:then_1
      (Variables|Default|SetMainWeapon NewWeapon))))

(fn GetMainWeapon
  (return (Variables|Default|GetMainWeapon)))

(fn SetCombatEnable
  (params (bIsCombatEnable? :type Boolean))
  (bind _output_get (Variables|Default|SetbIsCombatEnable? bIsCombatEnable?))
  (Default|CallOnToggleCombat _output_get) ; Dispatchers: Set Master AI Controller Blackboard Key bCombatEnable
)

(fn IsCombatEnable?
  (return (Variables|Default|GetbIsCombatEnable?)))

(fn ResetAttack
  (Variables|Default|SetAttackCount 0)
  (Variables|Default|SetbIsAttackSaved? false)
  (Variables|Default|SetbCanContinueAttack? false))